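; CustomizationCharacter is an interactable that randomizes the colors of the character that interacts with it.
; It shows its PressE prompt component when it becomes active and hides it when it stops being active.
; On interaction it calls ChangeColors on the interacting character, passing two random opaque colors and a random color balance.
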(event EventOnInteraction
  (params (Character :type Third%20Person%20Character%20Object%20Reference))
  (Default|ChangeColors Character (Utilities|Struct|MakeLinearColor (Math|Random|RandomFloat) (Math|Random|RandomFloat) (Math|Random|RandomFloat) 1.0) (Utilities|Struct|MakeLinearColor (Math|Random|RandomFloat) (Math|Random|RandomFloat) (Math|Random|RandomFloat) 1.0) (Math|Random|RandomFloatinRange 0.0 1.2)))

(event EventOnBecameActive
  (Rendering|SetVisibility (Variables|Default|GetPressE) true false))

(event EventOnStoppedActive
  (Rendering|SetVisibility (Variables|Default|GetPressE) false false))

(fn ConstructionScript)