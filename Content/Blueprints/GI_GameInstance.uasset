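; Game instance that signs the player into PlayFab through Steam and manages multiplayer session hosting and invite joining.
; After a short delay on Init, it logs in with a Steam auth ticket, creating an account if needed, and prints the result.
; CreateSession makes an advanced session and opens Asian_Village_Demo as a listen server.
; Accepted invites join the session, then issue a servertravel console command for that map.
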(event Custom|ConnectToPlayFab
  (|LoginwithSteam (Utilities|Struct|MakeClientLoginWithSteamRequest true 0 "" 0 "" (Class|PlayFabGameInstanceSubsystem|GetSteamAuthToken (Subsystems|GetPlayFabGameInstanceSubsystem))) (delegate Custom|OnSuccess) (delegate Custom|OnFailure)))

(event Custom|OnSuccess
  (params (result :type Client%20Login%20Result%20Structure) (customData :type Object%20Object%20Reference))
  (Development|PrintString "Connected" true true "(R=0.000000,G=0.660000,B=1.000000,A=1.000000)" 111.0))

(event Custom|OnFailure
  (params (error :type Play%20Fab%20Error%20Structure) (customData :type Object%20Object%20Reference))
  (bind (_haserror _errorcode _errorname _errormessage) (Utilities|Struct|BreakPlayFabError error))
  (Development|PrintString _errorname true true "(R=0.000000,G=0.660000,B=1.000000,A=1.000000)" 111.0)
  (Development|PrintString _errormessage true true "(R=0.000000,G=0.660000,B=1.000000,A=1.000000)" 111.0))

(event Custom|CreateSession
  (params (ExtraSettings :type Array%20of%20Session%20Property%20Key%20Pair%20Structures) (PublicConnections :type Integer))
  (|AdvancedSession ExtraSettings (Game|GetPlayerController 0) PublicConnections 0 false true false true true true false false false true false true
    (:OnSuccess
      (Development|PrintString "Session created")
      (Game|OpenLevel(byName) "Asian_Village_Demo" true "listen"))
    (:OnFailure
      (Development|PrintString "Session failed" true true "(R=0.000000,G=0.660000,B=1.000000,A=1.000000)" 111.0))))

(event Custom|Travel
  (params (MapName :type String))
  (Development|ExecuteConsoleCommand (Utilities|String|Append "servertravel " MapName) (Game|GetPlayerController 0)))

(event Custom|JoinToSession
  (params (SearchResult :type Blueprint%20Session%20Result%20Structure%20%28by%20ref%29))
  (|JoinSession (Game|GetPlayerController 0) SearchResult
    (:OnSuccess
      (CallFunction|Travel "Asian_Village_Demo"))))

(event EventInit
  (Utilities|FlowControl|Delay 2.0)
  (Class|PlayFabUtilities|SetPlayFabSettings "C8020")
  (CallFunction|ConnecttoPlayFab))

(event EventOnSessionInviteAccepted
  (params (LocalPlayerNum :type Integer) (PersonInvited :type BP%20Unique%20Net%20Id%20Structure) (SessionToJoin :type Blueprint%20Session%20Result%20Structure%20%28by%20ref%29))
  (CallFunction|JointoSession SessionToJoin))