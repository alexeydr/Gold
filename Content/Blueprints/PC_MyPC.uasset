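; Player controller that logs into PlayFab via Steam and manages coins, a leaderboard and server relays.
; A two-second loop queries Steam inventory (when flagged), tops up PlayFab AC from purchased coins, and broadcasts game coins plus donation balance (AC minus spent SC).
; The GlobalPoints leaderboard resolves Steam names through sequential account lookups before broadcasting.
; Event wrappers forward session hosting, bot movement and AI state changes to server events.
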(event Custom|AddPFCoins
  (params (Virtual%20Currency :type String) (Amount :type Integer))
  (|AddUserVirtualCurrency (Utilities|Struct|MakeClientAddUserVirtualCurrencyRequest Amount 0 Virtual%20Currency) (delegate Custom|CustomEvent) (EventDispatchers|CreateEvent :!event Custom|PlayfabErrorLog)))

(event Custom|AddGameCoins
  (params (Amount :type Integer))
  (CallFunction|AddPFCoins "GC" Amount))

(event Custom|OnItemsResultCompleted
  (bind _output_get (Variables|PlayfabData|SetAvailableCoins (- (Variables|PlayfabData|GetAc) (Variables|PlayfabData|GetSC))))
  (Default|CallOnCoinsCountUpdated (Variables|PlayfabData|GetGameCoins) _output_get)
  (Class|SteamInventory|DestroyResult (Class|SteamInventory|GetSteamInventory) (Variables|Default|GetResult%20Handle)))

(event Custom|PlayfabErrorLog
  (params (error :type Play%20Fab%20Error%20Structure) (customData :type Object%20Object%20Reference))
  (Development|PrintString (Utilities|Struct|BreakPlayFabError error) true true "(R=0.000000,G=0.660000,B=1.000000,A=1.000000)" 111.0))

(event Custom|ConnectToPlayFab
  (|LoginwithSteam (Utilities|Struct|MakeClientLoginWithSteamRequest true (Class|PlayFabGameInstanceSubsystem|GetSteamAuthToken (Subsystems|GetPlayFabGameInstanceSubsystem))) (delegate Custom|OnSuccess) (delegate Custom|OnFailure)
    (:OnPlayFabResponse
      (CallFunction|UpdateCoins :!label _label)
      (Utilities|FlowControl|Delay 2.0)
      (goto _label))))

(event Custom|GetCurrentCoinsCount
  (|GetUserInventory :onSuccess (delegate Custom|CustomEvent_0) :onFailure (EventDispatchers|CreateEvent :!event Custom|PlayfabErrorLog)))

(event Custom|CustomEvent_0
  (params (result :type Client%20Get%20User%20Inventory%20Result%20Structure) (customData :type Object%20Object%20Reference))
  (bind _virtualcurrency (Utilities|Struct|BreakClientGetUserInventoryResult result))
  (bind _allcoinscountsteam (Variables|Default|GetAllCoinsCountSteam))
  (for _array_element (Class|PlayFabJsonObject|GetFieldNames _virtualcurrency)
    (switch string _array_element
      (:AC
        (Variables|PlayfabData|SetAc (Math|Float|Truncate (Class|PlayFabJsonValue|AsNumber (Class|PlayFabJsonObject|GetField _virtualcurrency _array_element)))))
      (:SC
        (Variables|PlayfabData|SetSC (Math|Float|Truncate (Class|PlayFabJsonValue|AsNumber (Class|PlayFabJsonObject|GetField _virtualcurrency _array_element)))))
      (:GC
        (Variables|PlayfabData|SetGameCoins (Math|Float|Truncate (Class|PlayFabJsonValue|AsNumber (Class|PlayFabJsonObject|GetField _virtualcurrency _array_element)))))))
  (if (< (Variables|PlayfabData|GetAc) _allcoinscountsteam)
    (CallFunction|AddPFCoins "AC" (- _allcoinscountsteam (Variables|PlayfabData|GetAc)))
    (else
      (CallFunction|OnItemsResultCompleted))))

(event Custom|SubstractCoins
  (params (Amount :type Integer) (IsGameCoins :type Boolean))
  (if IsGameCoins
    (CallFunction|SubstractPFCoins Amount)
    (else
      (CallFunction|AddPFCoins "SC" Amount))))

(event Custom|OnSuccess
  (params (result :type Client%20Login%20Result%20Structure) (customData :type Object%20Object%20Reference))
  (Variables|Default|SetPlay%20Fab%20Id (Utilities|Struct|BreakClientLoginResult result))
  (Development|PrintString "Connected" true true "(R=0.000000,G=0.660000,B=1.000000,A=1.000000)" 111.0)
  (Audio|PlaySound2D "/Engine/EditorSounds/Notifications/CompileSuccess.CompileSuccess" 1.0 1.0 0.0 0 0))

(event Custom|OnFailure
  (params (error :type Play%20Fab%20Error%20Structure) (customData :type Object%20Object%20Reference))
  (bind (_haserror _errorcode _errorname _errormessage) (Utilities|Struct|BreakPlayFabError error))
  (Development|PrintString _errorname true true "(R=0.000000,G=0.660000,B=1.000000,A=1.000000)" 111.0)
  (Development|PrintString _errormessage true true "(R=0.000000,G=0.660000,B=1.000000,A=1.000000)" 111.0))

(event Custom|CustomEvent
  (params (result :type Client%20Modify%20User%20Virtual%20Currency%20Result%20Structure) (customData :type Object%20Object%20Reference))
  (CallFunction|UpdateCoins))

(event Custom|SubstractPFCoins
  (params (Amount :type Integer))
  (|SubtractUserVirtualCurrency (Utilities|Struct|MakeClientSubtractUserVirtualCurrencyRequest Amount 0 "GC") (delegate Custom|CustomEvent) (EventDispatchers|CreateEvent :!event Custom|PlayfabErrorLog)))

(event Custom|BuyCoins
  (params (Count :type Integer))
  (Class|AdvancedExternalUILibrary|ShowWebURLUI (Utilities|String|ToString(Text) (Utilities|Text|FormatText "https://store.steampowered.com/buyitem/{appid}/{itemdefid}/{quantity}" (Variables|Default|GetAppId) (Variables|ItemsIds|GetAllCoinsId) Count)) true false true 0 0 800 800))

(event Custom|OnInventoryFullUpdate
  (params (ResultHandle :type Steam%20Inventory%20Result%20Structure))
  (Variables|Default|SetResult%20Handle ResultHandle)
  (Utilities|FlowControl|Delay 0.2)
  (Variables|Default|SetAllCoinsCountSteam 0)
  (bind _itemsarray (Class|SteamInventory|GetResultItems (Class|SteamInventory|GetSteamInventory) (Variables|Default|GetResult%20Handle)))
  (for _array_element _itemsarray
    (CallFunction|SelectActionbyId _array_element))
  (CallFunction|GetCurrentCoinsCount))

(event Custom|OnResultUpdate
  (params (ResultHandle :type Steam%20Inventory%20Result%20Structure) (Result :type ESteamResult%20Enum :default "None"))
  (Variables|Default|SetResult%20Handle ResultHandle))

(event Custom|UpdateCoins
  ;[1 0 0 1 82] Crash in editor if true!!!
  (if (Variables|Default|GetNeedUpdateCoins)
    (bind _resulthandle (Class|SteamInventory|GetAllItems (Class|SteamInventory|GetSteamInventory)))
    (Variables|Default|SetResult%20Handle _resulthandle)))

(event Custom|ClientHostGame
  (params (ExtraSettings :type Array%20of%20Session%20Property%20Key%20Pair%20Structures))
  (CallFunction|ServerHostGame ExtraSettings))

(event Custom|ServerHostGame
  (params (ExtraSettings :type Array%20of%20Session%20Property%20Key%20Pair%20Structures))
  (bind _asgi_game_instance (Utilities|Casting|CastToGI_GameInstance (Game|GetGameInstance)))
  (Default|CreateSession _asgi_game_instance ExtraSettings))

(event EventBeginPlay
  (bind _returnvalue (Class|SteamInventory|GetSteamInventory))
  (|CallParentFunction)
  (EventDispatchers|BindEventtoMonSteamInventoryFullUpdate _returnvalue (EventDispatchers|CreateEvent :!event Custom|OnInventoryFullUpdate))
  (EventDispatchers|BindEventtoMonSteamInventoryResultReady _returnvalue (EventDispatchers|CreateEvent :!event Custom|OnResultUpdate))
  (CallFunction|ConnecttoPlayFab))

(event EventDestroyed
  (bind _returnvalue (Class|SteamInventory|GetSteamInventory))
  (EventDispatchers|UnbindallEventsfromMonSteamInventoryFullUpdate _returnvalue)
  (EventDispatchers|UnbindallEventsfromMonSteamInventoryResultReady _returnvalue)
  (|CallParentFunction))

(event Custom|CustomEvent_1
  (params (result :type Client%20Get%20Leaderboard%20Result%20Structure) (customData :type Object%20Object%20Reference))
  (bind _responseresult (Variables|Leaderboard|GetResponseResult))
  (Utilities|Array|Clear (Variables|Leaderboard|GetResponseResult))
  (Variables|Leaderboard|SetCurrentLeaderboardIndex 0)
  (for _array_element (.Leaderboard (Utilities|Struct|BreakClientGetLeaderboardResult result))
    (bind _returnvalue (Class|PlayFabJsonValue|AsObject (Class|PlayFabJsonObject|GetField _array_element "Profile")))
    (Utilities|Array|Add (Variables|Leaderboard|GetResponseResult) (Utilities|Struct|MakeBP_LeaderboardStructResult "" (Math|Float|Truncate (Class|PlayFabJsonValue|AsNumber (Class|PlayFabJsonObject|GetField _array_element "StatValue"))) (Class|PlayFabJsonValue|AsString (Class|PlayFabJsonObject|GetField _returnvalue "PlayerId")))))
  (if (Utilities|Array|IsValidIndex _responseresult (Variables|Leaderboard|GetCurrentLeaderboardIndex))
    (|GetAccountInfo (Utilities|Struct|MakeClientGetAccountInfoRequest "" (.PlayfabId (Utilities|Struct|BreakBP_LeaderboardStructResult (Utilities|Array|Get(acopy) _responseresult (Variables|Leaderboard|GetCurrentLeaderboardIndex))))) (delegate Custom|CustomEvent_8) (delegate Custom|CustomEvent_6))
    (else
      (Default|CallOnLeaderboardUpdated (Variables|Leaderboard|GetResponseResult)))))

(event Custom|CustomEvent_2
  (params (error :type Play%20Fab%20Error%20Structure) (customData :type Object%20Object%20Reference)))

(event Custom|CustomEvent_4
  (params (result :type Client%20Update%20Player%20Statistics%20Result%20Structure) (customData :type Object%20Object%20Reference)))

(event Custom|CustomEvent_8
  (params (result :type Client%20Get%20Account%20Info%20Result%20Structure) (customData :type Object%20Object%20Reference))
  (bind _responseresult (Variables|Leaderboard|GetResponseResult))
  (bind _returnvalue (Class|PlayFabJsonValue|AsObject (Class|PlayFabJsonObject|GetField (.AccountInfo (Utilities|Struct|BreakClientGetAccountInfoResult result)) "SteamInfo")))
  (Utilities|Struct|SetmembersinBP_LeaderboardStructResult (Utilities|Array|Get(acopy) (Variables|Leaderboard|GetResponseResult) (Variables|Leaderboard|GetCurrentLeaderboardIndex)) (Class|PlayFabJsonValue|AsString (Class|PlayFabJsonObject|GetField _returnvalue "SteamName")))
  (Math|Integer|IncrementInt (Variables|Leaderboard|GetCurrentLeaderboardIndex)
    (:%20%20
      (if (Utilities|Array|IsValidIndex _responseresult (Variables|Leaderboard|GetCurrentLeaderboardIndex))
        (|GetAccountInfo (Utilities|Struct|MakeClientGetAccountInfoRequest "" (.PlayfabId (Utilities|Struct|BreakBP_LeaderboardStructResult (Utilities|Array|Get(acopy) _responseresult (Variables|Leaderboard|GetCurrentLeaderboardIndex))))) (delegate Custom|CustomEvent_8) (delegate Custom|CustomEvent_6))
        (else
          (Default|CallOnLeaderboardUpdated (Variables|Leaderboard|GetResponseResult)))))))

(event Custom|CustomEvent_6
  (params (error :type Play%20Fab%20Error%20Structure) (customData :type Object%20Object%20Reference))
  (bind _responseresult (Variables|Leaderboard|GetResponseResult))
  (Math|Integer|IncrementInt (Variables|Leaderboard|GetCurrentLeaderboardIndex)
    (:%20%20
      (if (Utilities|Array|IsValidIndex _responseresult (Variables|Leaderboard|GetCurrentLeaderboardIndex))
        (|GetAccountInfo (Utilities|Struct|MakeClientGetAccountInfoRequest "" (.PlayfabId (Utilities|Struct|BreakBP_LeaderboardStructResult (Utilities|Array|Get(acopy) _responseresult (Variables|Leaderboard|GetCurrentLeaderboardIndex))))) (delegate Custom|CustomEvent_8) (delegate Custom|CustomEvent_6))
        (else
          (Default|CallOnLeaderboardUpdated (Variables|Leaderboard|GetResponseResult)))))))

(event Custom|GetCurrentsGlobalPoints
  (|GetLeaderboard (Utilities|Struct|MakeClientGetLeaderboardRequest 0 100 0 0 "GlobalPoints") (delegate Custom|CustomEvent_1) (delegate Custom|CustomEvent_2)))

(event Custom|AddGlobalPoints
  (params (Number :type Float%20%28single-precision%29))
  (bind _output_get (Variables|Leaderboard|SetLeaderboardJSON (Class|PlayFabJsonObject|ConstructJsonObject)))
  (Class|PlayFabJsonObject|SetStringField _output_get "StatisticName" "GlobalPoints")
  (Class|PlayFabJsonObject|SetField _output_get "Value" (Class|PlayFabJsonValue|ConstructJsonValueNumber Number))
  (|UpdatePlayerStatistics (Utilities|Struct|MakeClientUpdatePlayerStatisticsRequest 0 (Utilities|Array|MakeArray (Variables|Leaderboard|GetLeaderboardJSON))) (delegate Custom|CustomEvent_4) (delegate Custom|CustomEvent_2)))

(event Input|ActionEvents|InputActionLeaderboard
  (params (Key :type Key%20Structure))
  (:Pressed
    (Utilities|FlowControl|FlipFlop
      (:A
        (bind _returnvalue (UserInterface|CreateWidget "/Game/UI/Leaderboard/WBP_Leaderboard.WBP_Leaderboard_C"))
        (Variables|Leaderboard|SetLeaderboardWidget _returnvalue)
        (UserInterface|Viewport|AddtoViewport _returnvalue 0)
        (Variables|Default|SetbShowMouseCursor true)
        (Input|SetInputModeGameandUI 0 _returnvalue "DoNotLock" true false))
      (:B
        (Utilities|IsValid (Variables|Leaderboard|GetLeaderboardWidget)
          (:Is%20Valid
            (Widget|RemovefromParent (Variables|Leaderboard|GetLeaderboardWidget))
            (Variables|Default|SetbShowMouseCursor false)
            (Input|SetInputModeGameOnly self false)))))))

(event Input|ActionEvents|InputActionTestButton1
  (params (Key :type Key%20Structure))
  (:Pressed
    (CallFunction|AddGlobalPoints 2e+01)))

(event Custom|BotMoveToTableServer
  (params (AI :type BP%20Ai%20Object%20Reference) (Target%20Table :type BP%20Client%20Table%20Point%20Object%20Reference))
  (Default|MoveBot AI Target%20Table)
  (Default|SetBotontheTableClient Target%20Table AI))

(event Custom|BotMoveToTable
  (params (AI :type BP%20Ai%20Object%20Reference) (TargetTable :type BP%20Client%20Table%20Point%20Object%20Reference))
  (CallFunction|BotMovetoTableServer AI TargetTable))

(event Custom|BotMoveToActor
  (params (TargetActor :type Actor%20Object%20Reference) (Ai :type BP%20Ai%20Object%20Reference))
  (CallFunction|BotMovetoActorServer TargetActor Ai))

(event Custom|BotMoveToActorServer
  (params (TargetActor :type Actor%20Object%20Reference) (Ai :type BP%20Ai%20Object%20Reference))
  (Default|MoveBottoActor Ai TargetActor))

(event Custom|ClientDecreeseMentalState
  (params (Target :type BP%20Ai%20Object%20Reference) (Param :type Integer))
  (CallFunction|ServerDecreeseMentalState Target Param))

(event Custom|ServerDecreeseMentalState
  (params (Target :type BP%20Ai%20Object%20Reference) (Param :type Integer))
  (Variables|/Game/AI/BP_Ai.BP_Ai_C|SetMentalState Target (- (Variables|/Game/AI/BP_Ai.BP_Ai_C|GetMentalState Target) Param)))

(event Custom|ClientSetHaveTaskState
  (params (Target :type BP%20Ai%20Object%20Reference) (HaveTask :type Boolean))
  (CallFunction|ServerHaveTaskState Target HaveTask))

(event Custom|ServerHaveTaskState
  (params (Target :type BP%20Ai%20Object%20Reference) (HaveTask :type Boolean))
  (Variables|/Game/AI/BP_Ai.BP_Ai_C|SetHaveTask Target HaveTask))

(event Custom|ClientSetBotState
  (params (Target :type BP%20Ai%20Object%20Reference) (NewState :type BotStates%20Enum :default "NewEnumerator0"))
  (CallFunction|ServerSetBotState Target NewState))

(event Custom|ServerSetBotState
  (params (Target :type BP%20Ai%20Object%20Reference) (NewState :type BotStates%20Enum :default "NewEnumerator0"))
  (Variables|/Game/AI/BP_Ai.BP_Ai_C|SetCurrentState Target NewState))

(fn ConstructionScript)

(fn SelectActionbyId
  (params (SteamItemDetails :type Steam%20Item%20Details%20Structure%20%28by%20ref%29))
  (bind (_itemid _definition _quantity) (Utilities|Struct|BreakSteamItemDetails SteamItemDetails))
  (switch int (Utilities|Struct|BreakSteamItemDef _definition)
    (:100
      (Variables|Default|SetAllCoinsCountSteam (+ _quantity (Variables|Default|GetAllCoinsCountSteam))))))