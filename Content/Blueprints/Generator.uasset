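; Generator actor that stands as an early, unfinished level generator for destructible cubes.
; On BeginPlay it calls GenerateLevel, which spawns a single BP_DestructionCube at the actor's own location.
; Plane sizing derived from hub size divided by cube size, and a half-cube offset spawn, exist only as unreached logic.
; AddPlaneSizeInCubes does nothing, as its world-scale adjustment is disconnected.
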(event Custom|GenerateLevel
  (Game|SpawnActorfromClass "/Game/Blueprints/DestructionAssets/BP_DestructionCube.BP_DestructionCube_C" (Math|Transform|MakeTransform (Transformation|GetActorLocation) "0, 0, 0" "1.000000,1.000000,1.000000") "Undefined" 0 0 0))

(event EventBeginPlay
  (CallFunction|GenerateLevel))

(fn ConstructionScript)

(fn InitialPlaneSizeinHub
  (bind _hubsize (Variables|Default|GetHubSize))
  (bind _cubesize (Variables|Default|GetCubeSize))
  (bind _returnvalue (/ _hubsize _cubesize))
  (CallFunction|AddPlaneSizeinCubes (Math|Float|Truncate (.x _returnvalue)) (Math|Float|Truncate (.y _returnvalue))))

(fn AddPlaneSizeinCubes
  (params (InX :type Integer) (InY :type Integer)))