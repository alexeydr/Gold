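; Menu game mode that signs the player into PlayFab through Steam when play begins.
; On BeginPlay it takes the Steam auth token from the PlayFab game instance subsystem and sends a Steam login request that creates an account if none exists.
; Success prints a connected message and plays a sound, while failure prints the error name and message on screen.
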(event Custom|OnSuccess
  (params (result :type Client%20Login%20Result%20Structure) (customData :type Object%20Object%20Reference))
  (Development|PrintString "Connected" true true "(R=0.000000,G=0.660000,B=1.000000,A=1.000000)" 111.0)
  (Audio|PlaySound2D "/Engine/EditorSounds/Notifications/CompileSuccess.CompileSuccess" 1.0 1.0 0.0 0 0))

(event Custom|OnFailure
  (params (error :type Play%20Fab%20Error%20Structure) (customData :type Object%20Object%20Reference))
  (bind (_haserror _errorcode _errorname _errormessage) (Utilities|Struct|BreakPlayFabError error))
  (Development|PrintString _errorname true true "(R=0.000000,G=0.660000,B=1.000000,A=1.000000)" 111.0)
  (Development|PrintString _errormessage true true "(R=0.000000,G=0.660000,B=1.000000,A=1.000000)" 111.0))

(event EventBeginPlay
  (|CallParentFunction)
  (|LoginwithSteam (Utilities|Struct|MakeClientLoginWithSteamRequest true (Class|PlayFabGameInstanceSubsystem|GetSteamAuthToken (Subsystems|GetPlayFabGameInstanceSubsystem))) (delegate Custom|OnSuccess) (delegate Custom|OnFailure)))

(fn ConstructionScript)