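; BP_RecipesShop is an interactable shop actor in the restaurant that hosts a WBP_RecipesShop recipe store widget.
; On BeginPlay it passes itself to that widget, and a second widget is shown or hidden as the actor becomes active or inactive.
; Interaction toggles between shop and game, blending the view target, switching cursor and input mode, and showing or hiding the store, which refreshes on opening.
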(event Custom|ChangeTarget
  (if (Variables|Default|GetTargetOnWidget)
    (CallFunction|SetPlayerTargetonGame)
    (else
      (CallFunction|SetPlayerTargetonWiget)
      (bind _aswbp_recipes_shop (Utilities|Casting|CastToWBP_RecipesShop (UserInterface|GetWidget (Variables|Default|GetWidget1))))
      (Default|UpdateStore _aswbp_recipes_shop))))

(event EventOnInteraction
  (params (Character :type Third%20Person%20Character%20Object%20Reference))
  (CallFunction|ChangeTarget))

(event EventOnStoppedActive
  (Rendering|SetVisibility (Variables|Default|GetWidget) false false))

(event EventOnBecameActive
  (Rendering|SetVisibility (Variables|Default|GetWidget) true false))

(event EventBeginPlay
  (bind _aswbp_recipes_shop (Utilities|Casting|CastToWBP_RecipesShop (UserInterface|GetWidget (Variables|Default|GetWidget1))))
  (Variables|/Game/UI/RecipesShop/WBP_RecipesShop.WBP_RecipesShop_C|SetRecipeShop _aswbp_recipes_shop self))

(fn ConstructionScript)

(fn SetPlayerTargetonWiget
  (bind _returnvalue (Game|GetPlayerController 0))
  (bind _widget1 (Variables|Default|GetWidget1))
  (Variables|Default|SetTargetOnWidget true)
  (Game|Player|SetViewTargetwithBlend _returnvalue self 0.5 "VTBlend_Linear" 0.0 false)
  (Variables|/Script/Engine.PlayerController|SetbShowMouseCursor _returnvalue true)
  (Input|SetInputModeGameandUI _returnvalue (UserInterface|GetUserWidgetObject _widget1) "DoNotLock" true false)
  (Rendering|SetVisibility _widget1 true false))

(fn SetPlayerTargetonGame
  (bind _returnvalue (Game|GetPlayerController 0))
  (Variables|Default|SetTargetOnWidget false)
  (Game|Player|SetViewTargetwithBlend _returnvalue (Game|GetPlayerCharacter 0) 0.5 "VTBlend_Linear" 0.0 false)
  (Variables|/Script/Engine.PlayerController|SetbShowMouseCursor _returnvalue false)
  (Input|SetInputModeGameOnly _returnvalue false)
  (Rendering|SetVisibility (Variables|Default|GetWidget1) false false))