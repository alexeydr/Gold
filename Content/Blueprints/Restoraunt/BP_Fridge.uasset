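; Restaurant fridge actor that the player interacts with to view its items through a widget component.
; Interaction by player 0 while IsEmpty is set reports IsEmpty false through PC_MyPC, then toggles view mode.
; The toggle blends the camera between fridge and character, switches cursor, input mode and widget visibility, and refreshes items on opening.
; It also binds PC_MyPC's consume-start event to spawn a WBP_ApplyItems screen.
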(event Custom|OnConsumeStart_Event
  (params (AllItmes :type Integer))
  (bind _returnvalue (UserInterface|CreateWidget "/Game/UI/SmallInteractions/Friedge/WBP_ApplyItems.WBP_ApplyItems_C" 0 AllItmes))
  (UserInterface|Viewport|AddtoViewport _returnvalue 0))

(event Custom|ChangeTarget
  (if (Variables|Default|GetTargetOnWidget)
    (CallFunction|SetPlayerTargetonGame)
    (else
      (CallFunction|SetPlayerTargetonWiget)
      (bind _aswbp_friedge_widget (Utilities|Casting|CastToWBP_FriedgeWidget (UserInterface|GetUserWidgetObject (Variables|Default|GetWidget))))
      (Default|UpdateItems _aswbp_friedge_widget (Variables|Default|GetItems) self))))

(event EventBeginPlay
  (bind _aspc_my_pc (Utilities|Casting|CastToPC_MyPC (Game|GetPlayerController 0)))
  (EventDispatchers|AssignOnConsumeStart _aspc_my_pc (delegate Custom|OnConsumeStart_Event)))

(event EventOnInteraction
  (params (Character :type Third%20Person%20Character%20Object%20Reference))
  (if (and (== Character (Game|GetPlayerCharacter 0)) (Variables|Default|GetIsEmpty))
    (bind _aspc_my_pc (Utilities|Casting|CastToPC_MyPC (Game|GetPlayerController 0)))
    (Default|ClientFriegeEmpty _aspc_my_pc self false)
    (CallFunction|ChangeTarget)))

(fn ConstructionScript)

(fn SetPlayerTargetonWiget
  (bind _returnvalue (Game|GetPlayerController 0))
  (bind _widget (Variables|Default|GetWidget))
  (Variables|Default|SetTargetOnWidget true)
  (Game|Player|SetViewTargetwithBlend _returnvalue self 0.5 "VTBlend_Linear" 0.0 false)
  (Variables|/Script/Engine.PlayerController|SetbShowMouseCursor _returnvalue true)
  (Input|SetInputModeGameandUI _returnvalue (UserInterface|GetUserWidgetObject _widget) "DoNotLock" true false)
  (Rendering|SetVisibility _widget true false))

(fn SetPlayerTargetonGame
  (bind _returnvalue (Game|GetPlayerController 0))
  (Variables|Default|SetTargetOnWidget false)
  (Game|Player|SetViewTargetwithBlend _returnvalue (Game|GetPlayerCharacter 0) 0.5 "VTBlend_Linear" 0.0 false)
  (Variables|/Script/Engine.PlayerController|SetbShowMouseCursor _returnvalue false)
  (Input|SetInputModeGameOnly _returnvalue false)
  (Rendering|SetVisibility (Variables|Default|GetWidget) false false))