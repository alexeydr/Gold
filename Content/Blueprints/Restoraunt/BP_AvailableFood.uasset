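; Interactable restaurant actor that hosts an available-food widget for selecting recipes.
; Interaction toggles focus, blending the view between this actor and the player character while switching mouse cursor and input mode.
; Closing the widget returns focus to the game.
; Recipes selected in the widget are passed to every ThirdPersonCharacter as its selected items.
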(event Custom|OnClose_Event
  (CallFunction|SetPlayerTargetonGame))

(event Custom|CustomEvent
  (params (SelectedRecipes :type Array%20of%20Strings))
  (bind _outactors (Actor|GetAllActorsOfClass "/Game/ThirdPersonBP/Blueprints/ThirdPersonCharacter.ThirdPersonCharacter_C"))
  (for _array_element _outactors
    (Default|SetSelectedItems _array_element SelectedRecipes)))

(event Custom|ChangeTarget
  (if (Variables|Default|GetTargetOnWidget)
    (CallFunction|SetPlayerTargetonGame)
    (else
      (CallFunction|SetPlayerTargetonWiget))))

(event EventBeginPlay
  (|CallParentFunction)
  (bind _aswbp_available_food (Utilities|Casting|CastToWBP_AvailableFood (UserInterface|GetUserWidgetObject (Variables|Default|GetWidget))))
  (EventDispatchers|AssignOnClose _aswbp_available_food (delegate Custom|OnClose_Event))
  (EventDispatchers|BindEventtoOnRecipesSelected _aswbp_available_food (delegate Custom|CustomEvent)))

(event EventOnInteraction
  (params (Character :type Third%20Person%20Character%20Object%20Reference))
  (CallFunction|ChangeTarget))

(fn ConstructionScript)

(fn SetPlayerTargetonGame
  (bind _returnvalue (Game|GetPlayerController 0))
  (Variables|Default|SetTargetOnWidget false)
  (Game|Player|SetViewTargetwithBlend _returnvalue (Game|GetPlayerCharacter 0) 0.5 "VTBlend_Linear" 0.0 false)
  (Variables|/Script/Engine.PlayerController|SetbShowMouseCursor _returnvalue false)
  (Input|SetInputModeGameOnly _returnvalue false))

(fn SetPlayerTargetonWiget
  (bind _returnvalue (Game|GetPlayerController 0))
  (Variables|Default|SetTargetOnWidget true)
  (Game|Player|SetViewTargetwithBlend _returnvalue self 0.5 "VTBlend_Linear" 0.0 false)
  (Variables|/Script/Engine.PlayerController|SetbShowMouseCursor _returnvalue true)
  (Input|SetInputModeGameandUI _returnvalue (UserInterface|GetUserWidgetObject (Variables|Default|GetWidget)) "DoNotLock" true false))