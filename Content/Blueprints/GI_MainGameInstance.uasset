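; Game instance that sets up PlayFab and logs the player in through Steam when the game starts.
; On Init it applies the PlayFab title ID, waits a fixed delay, then logs in with a Steam auth token from the PlayFab game instance subsystem, allowing account creation.
; Login success and failure only print debug messages to screen, with failures showing the error name and message.
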(event Custom|ConnectToPlayFab
  (|LoginwithSteam (Utilities|Struct|MakeClientLoginWithSteamRequest true 0 "" 0 "" (Class|PlayFabGameInstanceSubsystem|GetSteamAuthToken (Subsystems|GetPlayFabGameInstanceSubsystem))) (delegate Custom|OnSuccess) (delegate Custom|OnFailure)))

(event Custom|OnSuccess
  (params (result :type Client%20Login%20Result%20Structure) (customData :type Object%20Object%20Reference))
  (Development|PrintString "Hello"))

(event Custom|OnFailure
  (params (error :type Play%20Fab%20Error%20Structure) (customData :type Object%20Object%20Reference))
  (bind (_haserror _errorcode _errorname _errormessage) (Utilities|Struct|BreakPlayFabError error))
  (Development|PrintString _errorname true true "(R=0.000000,G=0.660000,B=1.000000,A=1.000000)" 111.0)
  (Development|PrintString _errormessage true true "(R=0.000000,G=0.660000,B=1.000000,A=1.000000)" 111.0))

(event EventInit
  (Class|PlayFabUtilities|SetPlayFabSettings (Variables|Default|GetGame%20Title%20Id))
  (Utilities|FlowControl|Delay 5.0)
  (CallFunction|ConnecttoPlayFab))