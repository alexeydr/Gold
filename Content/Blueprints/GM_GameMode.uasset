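; Game mode that spawns AI customer bots for a venue with client tables.
; On BeginPlay it caches the first BotSpawn-tagged actor's location and starts a one-second looping spawn check.
; A bot spawns there only if no existing BP_Ai is in either of its first two states and HasEmptyTable finds a BP_ClientTablePoint without a valid bot.
; Each new bot then generates its clothing visuals.
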(event Custom|StartSpawnCharactersServer
  (Variables|Default|SetHasJustSpawnedBot false)
  (bind _outactors (Actor|GetAllActorsOfClass "/Game/AI/BP_Ai.BP_Ai_C"))
  (for _array_element _outactors
    (if (or (Utilities|Enum|Equal(Enum) (Variables|/Game/AI/BP_Ai.BP_Ai_C|GetCurrentState _array_element) "NewEnumerator0") (Utilities|Enum|Equal(Enum) (Variables|/Game/AI/BP_Ai.BP_Ai_C|GetCurrentState _array_element) "NewEnumerator1"))
      (Variables|Default|SetHasJustSpawnedBot true)))
  (if (and (not (Variables|Default|GetHasJustSpawnedBot)) (CallFunction|HasEmptyTable))
    (bind _returnvalue (AI|SpawnAIFromClass "/Game/AI/BP_Ai.BP_Ai_C" 0 (Variables|Default|GetSpawnLocation) "0, 0, 0" false 0))
    (bind _asbp_ai (Utilities|Casting|CastToBP_Ai _returnvalue))
    (CallFunction|ServerGenerateAiClothes _asbp_ai)))

(event Custom|StartSpawnCharacters
  (CallFunction|StartSpawnCharactersServer))

(event Custom|ServerGenerateAiClothes
  (params (Bot :type BP%20Ai%20Object%20Reference))
  (Default|GenerateAiVisual Bot))

(event EventBeginPlay
  (bind _outactors (Actor|GetAllActorswithTag "BotSpawn"))
  (Variables|Default|SetSpawnLocation (Transformation|GetActorLocation (Utilities|Array|Get(acopy) _outactors)))
  (Utilities|Time|SetTimerbyEvent (delegate Custom|StartSpawnCharacters) 1.0 true)
  (CallFunction|StartSpawnCharacters))

(fn ConstructionScript)

(fn HasEmptyTable
  (bind _outactors (Actor|GetAllActorsOfClass "/Game/Blueprints/Restoraunt/BP_ClientTablePoint.BP_ClientTablePoint_C"))
  (for _array_element _outactors
    (if (not (Utilities|IsValid (Variables|/Game/Blueprints/Restoraunt/BP_ClientTablePoint.BP_ClientTablePoint_C|GetBotOnTheTable _array_element)))
      (return true)))
  (return false))