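; Customer AI that gets seated, orders, eats and leaves, driven by player interaction and timed state changes.
; SetNewState routes state and task changes through PC_MyPC; spawn state opens a table menu with camera blend, and BP_AiController handles movement.
; A timer drains mental state in certain idle states, sending the customer out at zero.
; RepNotifies update the camera-facing mood widget and randomized modular outfit, which follows a leader pose.
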(event Custom|DecreesMentalState
  (bind _currentstate (Variables|Default|GetCurrentState))
  (if (not (Variables|Default|GetHaveTask))
    (if (and (Utilities|Enum|NotEqual(Enum) _currentstate "NewEnumerator3") (Utilities|Enum|NotEqual(Enum) _currentstate "NewEnumerator6"))
      (CallFunction|ServerDecreesMentalState))))

(event Custom|ReturnToPreviousState
  (CallFunction|SetTaskState false)
  (CallFunction|SetNewState (Utilities|Enum|ByteToEnumBotStates (- (Variables|Default|GetCurrentState) 1))))

(event Custom|Assign%20Meshes%20to%20same%20skeleton
  (Components|SkinnedMesh|SetLeaderPoseComponent (Variables|Default|GetSM_Cloth_CasualTop02) (Variables|Character|GetMesh) false false))

(event Custom|ExpelClient
  (CallFunction|SetTaskState false)
  (CallFunction|SetNewState "NewEnumerator2"))

(event Custom|SetNewState
  (params (Selection :type BotStates%20Enum :default "NewEnumerator0"))
  (if (not (Variables|Default|GetHaveTask))
    (CallFunction|SetTaskState true)
    (Default|ClientSetBotState (.AsPC%20My%20PC (Utilities|Casting|CastToPC_MyPC (Game|GetPlayerController 0))) self Selection)
    (switch Utilities|FlowControl|Switch|SwitchonBotStates Selection
      (:NewEnumerator0
        (CallFunction|SetTaskState false))
      (:NewEnumerator1
        (CallFunction|SetPlayerTargetonWiget))
      (:NewEnumerator2
        (Utilities|FlowControl|Delay (Variables|Default|GetSelectFoodTimer))
        (CallFunction|SetTaskState false)
        (CallFunction|SetNewState "NewEnumerator3"))
      (:NewEnumerator3
        (CallFunction|SetTaskState false)
        (Utilities|FlowControl|Delay (Variables|Default|GetWantedOrderTimer))
        (if (Utilities|Enum|Equal(Enum) (Variables|Default|GetCurrentState) "NewEnumerator3")
          (CallFunction|SetTaskState false)
          (CallFunction|SetNewState "NewEnumerator4")))
      (:NewEnumerator4
        (CallFunction|SetTaskState false))
      (:NewEnumerator5
        (Development|PrintString "Talk" true true "(R=1.000000,G=0.069442,B=0.000000,A=1.000000)" 11.0)
        (CallFunction|SetTaskState false)
        (CallFunction|SetNewState "NewEnumerator6"))
      (:NewEnumerator6
        (CallFunction|SetTaskState false)
        (Utilities|FlowControl|Delay (Variables|Default|GetWaitOrderTimer))
        (if (Utilities|Enum|Equal(Enum) (Variables|Default|GetCurrentState) "NewEnumerator6")
          (CallFunction|SetNewState "NewEnumerator7")))
      (:NewEnumerator7
        (CallFunction|SetTaskState false))
      (:NewEnumerator8
        (Development|PrintString "Eat" true true "(R=1.000000,G=0.069442,B=0.000000,A=1.000000)" 11.0)
        (Utilities|FlowControl|Delay (Variables|Default|GetEatingDelay))
        (CallFunction|SetTaskState false)
        (CallFunction|SetNewState "NewEnumerator9"))
      (:NewEnumerator9
        (CallFunction|MoveBottoExtractionPoint)))))

(event Custom|SetTaskState
  (params (HaveTask :type Boolean))
  (bind _aspc_my_pc (Utilities|Casting|CastToPC_MyPC (Game|GetPlayerController 0)))
  (Default|ClientSetHaveTaskState _aspc_my_pc self HaveTask))

(event Custom|OnPlayerInteractionWithTableMenu
  (params (SelectedTable :type BP%20Client%20Table%20Point%20Object%20Reference) (InteractionMenu :type TableInteractions%20Enum :default "NewEnumerator0"))
  (CallFunction|SetPlayerTargetonGame)
  (switch Utilities|FlowControl|Switch|SwitchonTableInteractions InteractionMenu
    (:NewEnumerator0
      (bind _aspc_my_pc (Utilities|Casting|CastToPC_MyPC (Game|GetPlayerController 0)))
      (Default|BotMovetoTable _aspc_my_pc self SelectedTable))
    (:NewEnumerator1
      (CallFunction|ExpelClient))
    (:NewEnumerator2
      (CallFunction|ReturntoPreviousState))))

(event Custom|ServerDecreesMentalState
  (Variables|Default|SetMentalState (- (Variables|Default|GetMentalState) 1)))

(event EventOnBecameActive
  (Rendering|SetVisibility (Variables|Default|GetPressE) true false))

(event EventOnStoppedActive
  (Rendering|SetVisibility (Variables|Default|GetPressE) false false))

(event EventOnInteraction
  (params (Character :type Third%20Person%20Character%20Object%20Reference))
  (if (Utilities|Enum|Equal(Enum) (Variables|Default|GetCurrentState) "NewEnumerator3")
    (CallFunction|SetNewState "NewEnumerator5")
    (elif (Utilities|Enum|Equal(Enum) (Variables|Default|GetCurrentState) "NewEnumerator6")
      (CallFunction|SetNewState "NewEnumerator8")
      (else
        (CallFunction|SetNewState (Utilities|Enum|ByteToEnumBotStates (+ (Variables|Default|GetCurrentState) 1)))))))

(event EventTick
  (params (DeltaSeconds :type Float%20%28single-precision%29))
  (bind _returnvalue (Game|GetPlayerCameraManager 0))
  (bind _mentalwidget (Variables|Default|GetMentalWidget))
  (|CallParentFunction DeltaSeconds)
  (Utilities|IsValid _mentalwidget
    (:Is%20Valid
      (Utilities|IsValid _returnvalue
        (:Is%20Valid
          (Transformation|SetWorldRotation _mentalwidget (Math|Rotator|FindLookatRotation (Transformation|GetWorldLocation _mentalwidget) (Transformation|GetActorLocation _returnvalue)) false false))))))

(event EventBeginPlay
  (|CallParentFunction)
  (Utilities|Time|SetTimerbyEvent (delegate Custom|DecreesMentalState) (Variables|Default|GetDecressMentalTime) true)
  (bind _aswbp_main_client_widget (Utilities|Casting|CastToWBP_MainClientWidget (UserInterface|GetWidget (Variables|Default|GetWidget))))
  (EventDispatchers|BindEventtoOnTableMenuInteraction (Variables|/Game/UI/ClientWidgets/WBP_MainClientWidget.WBP_MainClientWidget_C|GetWBP_TableManagement _aswbp_main_client_widget) (EventDispatchers|CreateEvent :!event Custom|OnPlayerInteractionWithTableMenu)))

(event Custom|MoveBot
  (params (TargetTable :type BP%20Client%20Table%20Point%20Object%20Reference))
  (bind _asbp_ai_controller (Utilities|Casting|CastToBP_AiController (Pawn|GetController)))
  (Default|MovetoTable _asbp_ai_controller TargetTable))

(event Custom|MoveBotToActor
  (params (TargetActor :type Actor%20Object%20Reference))
  (bind _asbp_ai_controller (Utilities|Casting|CastToBP_AiController (Pawn|GetController)))
  (Default|BotMovetoActor _asbp_ai_controller TargetActor))

(event Custom|MoveBotToExtractionPoint
  (bind _aspc_my_pc (Utilities|Casting|CastToPC_MyPC (Game|GetPlayerController 0)))
  (bind _returnvalue (Actor|GetActorOfClass "/Game/AI/BP_AiDestroyer.BP_AiDestroyer_C"))
  (Default|BotMovetoActor _aspc_my_pc _returnvalue self))

(fn ConstructionScript
  (CallFunction|AssignMeshestoSameSkeleton))

(fn SetPlayerTargetonWiget
  (bind _returnvalue (Game|GetPlayerController 0))
  (Game|Player|SetViewTargetwithBlend _returnvalue self 0.5 "VTBlend_Linear" 0.0 false)
  (Variables|/Script/Engine.PlayerController|SetbShowMouseCursor _returnvalue true)
  (Input|SetInputModeGameandUI _returnvalue (UserInterface|GetUserWidgetObject (Variables|Default|GetWidget)) "DoNotLock" true false)
  (Rendering|SetVisibility (Variables|Default|GetWidget) true false))

(fn SetPlayerTargetonGame
  (bind _returnvalue (Game|GetPlayerController 0))
  (Game|Player|SetViewTargetwithBlend _returnvalue (Game|GetPlayerCharacter 0) 0.5 "VTBlend_Linear" 0.0 false)
  (Variables|/Script/Engine.PlayerController|SetbShowMouseCursor _returnvalue false)
  (Input|SetInputModeGameOnly _returnvalue false)
  (Rendering|SetVisibility (Variables|Default|GetWidget) false false))

(fn GenerateAiVisual
  (Rendering|SetVisibility (Variables|Default|GetSM_Glasses) (<= (Math|Random|RandomFloatinRange 0.0 1.0) (LocalVariables|GetChanceOnGlass)) false)
  (Variables|Default|SetHairMesh (select (Math|Random|RandomBool) "/Game/GR_Stylized_Female_01/Character/Meshes/HAIR_Bobcut/SM_Hair_Bobcut.SM_Hair_Bobcut" "/Game/GR_Stylized_Female_01/Character/Meshes/HAIR_Ponytail/SM_Hair_Ponytail.SM_Hair_Ponytail"))
  (Variables|Default|SetShortMesh (Utilities|Select :Index (Math|Random|RandomIntegerinRange 0 4) :Option%200 "/Game/GR_Stylized_Female_01/Character/Meshes/CLOTH_Shorts_01/SM_Cloth_Shorts01.SM_Cloth_Shorts01" :Option%201 "/Game/GR_Stylized_Female_01/Character/Meshes/CLOTH_Casual_Shorts_01b/SM_Cloth_CasualsShorts01b.SM_Cloth_CasualsShorts01b" :Option%202 "/Game/GR_Stylized_Female_01/Character/Meshes/CLOTH_Sailor_Bottom_B/SM_Cloth_SailorBottomB_NOS.SM_Cloth_SailorBottomB_NOS" :Option%203 "/Game/GR_Stylized_Female_01/Character/Meshes/CLOTH_Pants/SM_Cloth_Pants.SM_Cloth_Pants" :Option%204 "/Game/GR_Stylized_Female_01/Character/Meshes/CLOTH_Underwear_01b_Bottom/SM_Cloth_Underwear01b_Bottom.SM_Cloth_Underwear01b_Bottom" :Option%205 0))
  (Variables|Default|SetTopMesh (Utilities|Select :Index (Math|Random|RandomIntegerinRange 0 4) :Option%200 "/Game/GR_Stylized_Female_01/Character/Meshes/CLOTH_Casual_Shirt_01b/SM_Cloth_CasualShirt01b.SM_Cloth_CasualShirt01b" :Option%201 "/Game/GR_Stylized_Female_01/Character/Meshes/CLOTH_Casual_Top_01/SM_Cloth_CasualTop01.SM_Cloth_CasualTop01" :Option%202 "/Game/GR_Stylized_Female_01/Character/Meshes/CLOTH_Casual_Top_02/SM_Cloth_CasualTop02.SM_Cloth_CasualTop02" :Option%203 "/Game/GR_Stylized_Female_01/Character/Meshes/CLOTH_sailor_top/SM_Cloth_SailorTopA_NOS.SM_Cloth_SailorTopA_NOS" :Option%204 "/Game/GR_Stylized_Female_01/Character/Meshes/CLOTH_Underwear_01_top/SM_Cloth_Underwear01_Top.SM_Cloth_Underwear01_Top")))

(fn OnRepHairMesh
  (Components|SkeletalMesh|SetSkeletalMeshAsset (Variables|Default|GetSM_Hair) (Variables|Default|GetHairMesh)))

(fn OnRepShortMesh
  (Components|SkeletalMesh|SetSkeletalMeshAsset (Variables|Default|GetSM_Cloth_Shorts01) (Variables|Default|GetShortMesh)))

(fn OnRepTopMesh
  (Components|SkeletalMesh|SetSkeletalMeshAsset (Variables|Default|GetSM_Cloth_CasualTop02) (Variables|Default|GetTopMesh)))

(fn OnRepMentalState
  (bind _mentalstate (Variables|Default|GetMentalState))
  (if (<= _mentalstate 0)
    (CallFunction|SetNewState "NewEnumerator9")
    (else
      (bind _aswbp_ai_mental_state (Utilities|Casting|CastToWBP_AiMentalState (UserInterface|GetWidget (Variables|Default|GetMentalWidget))))
      (Default|SetNewMentalValue _aswbp_ai_mental_state _mentalstate (Variables|Default|GetCurrentState)))))

(fn OnRepCurrentState
  (bind _aswbp_ai_mental_state (Utilities|Casting|CastToWBP_AiMentalState (UserInterface|GetWidget (Variables|Default|GetMentalWidget))))
  (Default|SetNewMentalValue _aswbp_ai_mental_state (Variables|Default|GetMentalState) (Variables|Default|GetCurrentState)))